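; BP_Door is a locked door that destroys itself to open once a key is held and shows the WB_controls widget.
; StartInteract checks the door's own HasKey, set by PickupKey, then either opens with a sound or shows WB_NOKEY for five seconds.
; A box overlap instead checks the cached first-person character's HasKey and opens silently through a DoOnce into OpenDoorTest.
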(event `OpenDoorTest`
  (bind _returnvalue (`|CreateWidget` "/Game/Blueprint/WB_controls.WB_controls_C"))
  (`UserWidget.AddToViewport` _returnvalue 0)
  (`self.K2_DestroyActor`))

(event `self.ReceiveBeginPlay`
  (bind _asbp_first_person_character (cast `/Game/FirstPerson/Blueprints/BP_FirstPersonCharacter` (`GameplayStatics.GetPlayerCharacter` 0)))
  (set `self.As BP First Person Character` _asbp_first_person_character))

(event `/Game/Blueprint/BPI_Interact.StartInteract`
  (if (`self.Has Key?`)
    (`GameplayStatics.PlaySoundAtLocation` "/Game/sounds/freesound_community-pick-hitting-rock-87562.freesound_community-pick-hitting-rock-87562" (`SceneComponent.GetSocketLocation` (`self.Door`) "None") (struct) 1.0 1.0 0.0 null null null null)
    (`self.K2_DestroyActor`)
    (cast `/Game/FirstPerson/Blueprints/BP_FirstPersonCharacter` (`GameplayStatics.GetPlayerCharacter` 0))
    (bind _returnvalue (`|CreateWidget` "/Game/Blueprint/WB_controls.WB_controls_C"))
    (`UserWidget.AddToViewport` _returnvalue 0)
    (else
      (cast `/Game/FirstPerson/Blueprints/BP_FirstPersonCharacter` (`GameplayStatics.GetPlayerCharacter` 0))
      (bind _returnvalue_2 (`|CreateWidget` "/Game/Blueprint/WB_NOKEY.WB_NOKEY_C"))
      (`UserWidget.AddToViewport` _returnvalue_2 0)
      (`KismetSystemLibrary.Delay` 5.0)
      (`WidgetBlueprintLibrary.GetAllWidgetsOfClass` "/Game/Blueprint/WB_NOKEY.WB_NOKEY_C")
      (`Widget.RemoveFromParent` _returnvalue_2))))

(event `/Game/Blueprint/BPI_Pickupkey.Pickup key`
  (set `self.Has Key?` true))

(event `self.Box.OnComponentBeginOverlap`
  (params (OverlappedComponent :type "PrimitiveComponent Object Reference") (OtherActor :type "Actor Object Reference") (OtherComp :type "PrimitiveComponent Object Reference") (OtherBodyIndex :type Integer) (bFromSweep :type Boolean) (SweepResult :type "HitResult Structure (by ref)"))
  (bind _as_bp_first_person_character (`self.As BP First Person Character`))
  (if (== OtherActor _as_bp_first_person_character)
    (if (== (`/Game/FirstPerson/Blueprints/BP_FirstPersonCharacter.Has Key?` _as_bp_first_person_character) true)
      (`/Engine/EditorBlueprintResources/StandardMacros.DoOnce` false
        (:`Completed`
          (`self.OpenDoorTest`))))))

(fn `UserConstructionScript`)
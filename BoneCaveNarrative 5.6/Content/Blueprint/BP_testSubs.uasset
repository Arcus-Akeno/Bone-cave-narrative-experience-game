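; Test pickup actor, apparently a key, that notifies a Door and shows on-screen widgets.
; Any overlap with its Box adds a new WB_Test widget to the viewport, with no filtering.
; StartInteract calls PickupKeyMessage on the Door, then, if the player is BP_FirstPersonCharacter, shows WB_LeTrumpReference and hides the actor.
; After a short delay it removes that widget and destroys itself.
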(event `self.Box.OnComponentBeginOverlap`
  (params (OverlappedComponent :type "PrimitiveComponent Object Reference") (OtherActor :type "Actor Object Reference") (OtherComp :type "PrimitiveComponent Object Reference") (OtherBodyIndex :type Integer) (bFromSweep :type Boolean) (SweepResult :type "HitResult Structure (by ref)"))
  (if true
    (bind _returnvalue (`|CreateWidget` "/Game/Blueprint/WB_Test.WB_Test_C"))
    (`UserWidget.AddToViewport` _returnvalue 0)))

(event `/Game/Blueprint/BPI_Interact.StartInteract`
  (message `/Game/Blueprint/BPI_Pickupkey.Pickup key` (`self.Door`))
  (cast `/Game/FirstPerson/Blueprints/BP_FirstPersonCharacter` (`GameplayStatics.GetPlayerCharacter` 0))
  (bind _returnvalue (`|CreateWidget` "/Game/Blueprint/WB_LeTrumpReference.WB_LeTrumpReference_C"))
  (`UserWidget.AddToViewport` _returnvalue 0)
  (`self.SetActorHiddenInGame` true)
  (`KismetSystemLibrary.Delay` 4.0)
  (`WidgetBlueprintLibrary.GetAllWidgetsOfClass` "/Game/Blueprint/WB_LeTrumpReference.WB_LeTrumpReference_C")
  (`Widget.RemoveFromParent` _returnvalue)
  (`self.K2_DestroyActor`))

(fn `UserConstructionScript`)
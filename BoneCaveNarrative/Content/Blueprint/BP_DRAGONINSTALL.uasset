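; BP_DRAGONINSTALL is an actor that performs a one-time "Dragon Install" transformation, a nod to Guilty Gear, once a trigger is activated.
; Every Tick it looks up all BP_Trigger actors and checks the Trigger flag on the first one.
; When that flag is true, a DoOnce spawns an enlarged explosion at its StaticMesh, plays the Dragon Install theme in 2D and swaps the mesh material.
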(event `self.ReceiveTick`
  (params (DeltaSeconds :type "Float (single-precision)"))
  (bind _outactors (`GameplayStatics.GetAllActorsOfClass` "/Game/Blueprint/BP_Trigger.BP_Trigger_C"))
  (if (`/Game/Blueprint/BP_Trigger.Trigger` (`|GetArrayItem` _outactors))
    (`/Engine/EditorBlueprintResources/StandardMacros.DoOnce` false
      (:`Completed`
        (`GameplayStatics.SpawnEmitterAtLocation` "/Game/StarterContent/Particles/P_Explosion.P_Explosion" (`SceneComponent.K2_GetComponentLocation` (`self.StaticMesh`)) (struct) (10.0 10.0 10.0) false)
        (`GameplayStatics.PlaySound2D` "/Game/Sounds/Guilty_Gear_Xrd_Sign_Original_Soundtrack_-_Ride_the_Fire___Dragon_Install_theme_.Guilty_Gear_Xrd_Sign_Original_Soundtrack_-_Ride_the_Fire___Dragon_Install_theme_" 1.0 1.0 0.0 null null)
        (`PrimitiveComponent.SetMaterial` (`self.StaticMesh`) 0 "/Game/M_DRAGONINSTALL.M_DRAGONINSTALL")))))

(fn `UserConstructionScript`)
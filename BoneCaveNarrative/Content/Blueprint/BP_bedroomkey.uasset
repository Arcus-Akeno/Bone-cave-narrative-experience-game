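; Bedroom key pickup actor that notifies its referenced Door when the player interacts with it.
; StartInteract calls PickupKeyMessage on the Door, then, if the player is a BP_FirstPersonCharacter, shows a WB_GETKEYbedroom widget and hides the key.
; After a four-second delay it removes the widget and destroys itself.
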(event `/Game/Blueprint/BPI_Interact.StartInteract`
  (message `/Game/Blueprint/BPI_Pickupkey.Pickup key` (`self.door`))
  (cast `/Game/FirstPerson/Blueprints/BP_FirstPersonCharacter` (`GameplayStatics.GetPlayerCharacter` 0))
  (bind _returnvalue (`|CreateWidget` "/Game/Blueprint/WB_GETKEYbedroom.WB_GETKEYbedroom_C"))
  (`UserWidget.AddToViewport` _returnvalue 0)
  (`self.SetActorHiddenInGame` true)
  (`KismetSystemLibrary.Delay` 4.0)
  (`WidgetBlueprintLibrary.GetAllWidgetsOfClass` "/Game/Blueprint/WB_GETKEYbedroom.WB_GETKEYbedroom_C")
  (`Widget.RemoveFromParent` _returnvalue)
  (`self.K2_DestroyActor`))

(fn `UserConstructionScript`)
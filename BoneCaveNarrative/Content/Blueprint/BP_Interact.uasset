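; BP_Interact is a prototype interaction zone that tracks whether something is inside its Box component.
; The box's begin and end overlap events set the Inarea flag, with no check on which actor overlaps.
; A custom event, apparently meant for an F key press though no caller appears here, tests that flag.
; Every outcome is only a debug string print, with no actual interaction yet.
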(event `self.Box.OnComponentBeginOverlap`
  (params (OverlappedComponent :type "PrimitiveComponent Object Reference") (OtherActor :type "Actor Object Reference") (OtherComp :type "PrimitiveComponent Object Reference") (OtherBodyIndex :type Integer) (bFromSweep :type Boolean) (SweepResult :type "HitResult Structure (by ref)"))
  (set `self.Inarea` true)
  (`KismetSystemLibrary.PrintString` "in area"))

(event `self.Box.OnComponentEndOverlap`
  (params (OverlappedComponent :type "PrimitiveComponent Object Reference") (OtherActor :type "Actor Object Reference") (OtherComp :type "PrimitiveComponent Object Reference") (OtherBodyIndex :type Integer))
  (set `self.Inarea` false)
  (`KismetSystemLibrary.PrintString` "out of area"))

(event `CustomEvent`
  (`KismetSystemLibrary.PrintString` "clicking  F")
  (if (`self.Inarea`)
    (`KismetSystemLibrary.PrintString` "working")
    (else
      (`KismetSystemLibrary.PrintString` "you fucked up"))))

(fn `UserConstructionScript`)
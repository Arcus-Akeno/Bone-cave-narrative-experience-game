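; BP_Pickaxe is a pickup actor that acts as a key for the first-person character.
; Overlapping its Box with the player sets HasKey on the character and destroys the actor.
; StartInteract instead calls PickupKeyMessage on a Door reference and destroys itself.
; A separate CustomEvent sends that message, hides the actor, shows the WB_GETKEYbedroom widget briefly, then removes both.
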(event `self.ReceiveBeginPlay`
  (bind _asbp_first_person_character (cast `/Game/FirstPerson/Blueprints/BP_FirstPersonCharacter` (`GameplayStatics.GetPlayerCharacter` 0)))
  (set `self.As BP First Person Character` _asbp_first_person_character))

(event `PickupKey`
  (set `/Game/FirstPerson/Blueprints/BP_FirstPersonCharacter.Has Key?` true (`self.As BP First Person Character`))
  (`self.K2_DestroyActor`))

(event `self.Box.OnComponentBeginOverlap`
  (params (OverlappedComponent :type "PrimitiveComponent Object Reference") (OtherActor :type "Actor Object Reference") (OtherComp :type "PrimitiveComponent Object Reference") (OtherBodyIndex :type Integer) (bFromSweep :type Boolean) (SweepResult :type "HitResult Structure (by ref)"))
  (if (== OtherActor (`self.As BP First Person Character`))
    (`self.PickupKey`)
    (`self.K2_DestroyActor`)))

(event `/Game/Blueprint/BPI_Interact.StartInteract`
  (message `/Game/Blueprint/BPI_Pickupkey.Pickup key` (`self.Door`))
  (`self.K2_DestroyActor`))

(event `CustomEvent`
  (message `/Game/Blueprint/BPI_Pickupkey.Pickup key` (`self.door`))
  (cast `/Game/FirstPerson/Blueprints/BP_FirstPersonCharacter` (`GameplayStatics.GetPlayerCharacter` 0))
  (bind _returnvalue (`|CreateWidget` "/Game/Blueprint/WB_GETKEYbedroom.WB_GETKEYbedroom_C"))
  (`UserWidget.AddToViewport` _returnvalue 0)
  (`self.SetActorHiddenInGame` true)
  (`KismetSystemLibrary.Delay` 4.0)
  (`WidgetBlueprintLibrary.GetAllWidgetsOfClass` "/Game/Blueprint/WB_GETKEYbedroom.WB_GETKEYbedroom_C")
  (`Widget.RemoveFromParent` _returnvalue)
  (`self.K2_DestroyActor`))

(fn `UserConstructionScript`)